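; Player-drivable tank Blueprint that wires its components together and maps input to driving, aiming and firing.
; BeginPlay registers the barrel and turret references and initialises TankMovement with both tracks.
; Forward and backward axes feed movement intent to TankMovement, while separate throttle axes drive each track directly.
; Aim axes rotate an azimuth gimbal and spring arm scaled by delta time, and the Fire action calls Fire.
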(event EventBeginPlay
  (Class|Tank|SetBarrelReference (Variables|Default|GetBarrel))
  (Class|Tank|SetTurretReference (Variables|Default|GetTurret))
  (Class|TankMovementComponent|Initialise (Variables|Default|GetTankMovement) (Variables|Default|GetTankTrackLeft) (Variables|Default|GetTankTrackRight)))

(event Input|ActionEvents|InputActionFire
  (params (Key :type Key%20Structure :default "AnyKey"))
  ;[1 1 1] Input
  (:Pressed
    (Class|Tank|Fire)))

(event Input|AxisEvents|InputAxisAimAzimuth
  (params (AxisValue :type Float%20%28single-precision%29))
  ;[1 1 1] Input
  (Transformation|AddLocalRotation (Variables|Default|GetAzimuth%20gibmle) (Math|Rotator|MakeRotator 0.0 0.0 (* AxisValue (Utilities|Time|GetWorldDeltaSeconds) 1e+02)) false false))

(event Input|AxisEvents|InputAxisMoveBackward
  (params (AxisValue :type Float%20%28single-precision%29))
  ;[1 1 1] Input
  (Class|TankMovementComponent|IntendMoveForward (Variables|Default|GetTankMovement) (* AxisValue -1.0)))

(event Input|AxisEvents|InputAxisMoveForward
  (params (AxisValue :type Float%20%28single-precision%29))
  ;[1 1 1] Input
  (Class|TankMovementComponent|IntendMoveForward (Variables|Default|GetTankMovement) AxisValue))

(event Input|AxisEvents|InputAxisLeftTrackThrottle
  (params (AxisValue :type Float%20%28single-precision%29))
  ;[1 1 1] Input
  (Class|TankTrack|SetThrottle (Variables|Default|GetTankTrackLeft) AxisValue))

(event Input|AxisEvents|InputAxisRightTrackThrottle
  (params (AxisValue :type Float%20%28single-precision%29))
  ;[1 1 1] Input
  (Class|TankTrack|SetThrottle (Variables|Default|GetTankTrackRight) AxisValue))

(event Input|AxisEvents|InputAxisAimElevation
  (params (AxisValue :type Float%20%28single-precision%29))
  ;[1 1 1] Input
  (Transformation|AddLocalRotation (Variables|Default|GetSpringArm) (Math|Rotator|MakeRotator 0.0 (* (Utilities|Time|GetWorldDeltaSeconds) AxisValue 1e+02) 0.0) false false))

(fn ConstructionScript)